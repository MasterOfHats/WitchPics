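; BP_PlaceholderCC is a placeholder player character controller providing basic movement, look and jump.
; Move axes feed flattened, normalized control-rotation forward and right vectors into the movement component, so pitch does not affect walking speed.
; Look axes drive controller yaw and pitch.
; Jump launches the character upward by JumpImpulse, only while the movement component reports walking, instead of using the built-in jump.
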(event EventBeginPlay)

(event Collision|EventActorBeginOverlap
  (params (OtherActor :type Actor%20Object%20Reference)))

(event EventTick
  (params (DeltaSeconds :type Float%20%28single-precision%29)))

(event Input|ActionEvents|InputActionJump
  (params (Key :type Key%20Structure :default "None"))
  (:Pressed
    (if (Pawn|Components|CharacterMovement|IsWalking (Variables|Character|GetCharacterMovement))
      (Character|LaunchCharacter (Math|Vector|MakeVector 0.0 0.0 (Variables|Default|GetJumpImpulse)) false false))))

(event Input|AxisEvents|InputAxisMoveForward
  (params (AxisValue :type Float%20%28single-precision%29))
  (Class|PawnMovementComponent|AddInputVector (Variables|Character|GetCharacterMovement) (* (Class|KismetMathLibrary|VectorNormal2D (Math|Vector|GetForwardVector (Pawn|GetControlRotation :!class /Script/Engine.Pawn)) 0.0001) AxisValue) false))

(event Input|AxisEvents|InputAxisMoveRight
  (params (AxisValue :type Float%20%28single-precision%29))
  (Class|PawnMovementComponent|AddInputVector (Variables|Character|GetCharacterMovement) (* (Class|KismetMathLibrary|VectorNormal2D (Math|Vector|GetRightVector (Pawn|GetControlRotation :!class /Script/Engine.Pawn)) 0.0001) AxisValue) false))

(event Input|AxisEvents|InputAxisLookRight
  (params (AxisValue :type Float%20%28single-precision%29))
  (Pawn|Input|AddControllerYawInput AxisValue))

(event Input|AxisEvents|InputAxisLookUp
  (params (AxisValue :type Float%20%28single-precision%29))
  (Pawn|Input|AddControllerPitchInput AxisValue))

(fn ConstructionScript)