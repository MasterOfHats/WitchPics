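; BP_Witch is a player-controlled pawn with axis-driven movement, mouse-look style yaw and pitch, and a sprint.
; Move input follows the control rotation's forward and right vectors, normalized in 2D and scaled by Acceleration, and feeds SimplePawnMovement as input vectors.
; Look axes drive controller yaw and pitch directly.
; Holding Left Shift sharply raises the movement component's maximum horizontal speed, and releasing it sets the slower speed.
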(event Input|ActionEvents|InputActionJump
  (params (Key :type Key%20Structure :default "None")))

(event Input|AxisEvents|InputAxisMoveForward
  (params (AxisValue :type Float%20%28single-precision%29))
  (Class|PawnMovementComponent|AddInputVector (Variables|Default|GetSimplePawnMovement) (* (Class|KismetMathLibrary|VectorNormal2D (Math|Vector|GetForwardVector (Pawn|GetControlRotation :!class /Script/Engine.Pawn)) 0.0001) AxisValue (Variables|Default|GetAcceleration)) false))

(event Input|AxisEvents|InputAxisMoveRight
  (params (AxisValue :type Float%20%28single-precision%29))
  (Class|PawnMovementComponent|AddInputVector (Variables|Default|GetSimplePawnMovement) (* (Class|KismetMathLibrary|VectorNormal2D (Math|Vector|GetRightVector (Pawn|GetControlRotation :!class /Script/Engine.Pawn)) 0.0001) AxisValue (Variables|Default|GetAcceleration)) false))

(event Input|AxisEvents|InputAxisLookRight
  (params (AxisValue :type Float%20%28single-precision%29))
  (Pawn|Input|AddControllerYawInput AxisValue))

(event Input|AxisEvents|InputAxisLookUp
  (params (AxisValue :type Float%20%28single-precision%29))
  (Pawn|Input|AddControllerPitchInput AxisValue))

(event Input|KeyboardEvents|LeftShift
  (params (Key :type Key%20Structure :default "None"))
  (bind _simplepawnmovement (Variables|Default|GetSimplePawnMovement))
  (:Pressed
    (Variables|/Script/LucidMovement.SimplePawnMovement|SetMaxHorizontalSpeed _simplepawnmovement 1e+04))
  (:Released
    (Variables|/Script/LucidMovement.SimplePawnMovement|SetMaxHorizontalSpeed _simplepawnmovement 9e+02)))

(fn ConstructionScript)